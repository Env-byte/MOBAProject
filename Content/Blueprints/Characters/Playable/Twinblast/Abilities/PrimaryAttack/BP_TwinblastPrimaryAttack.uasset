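; Gameplay ability for Twinblast's primary attack, which damages the character's current primary attack target.
; Activation caches the Twinblast character and commits; execution then turns the character toward the target's yaw.
; It applies a damage gameplay effect to the target's ability system through the CanTakeDamage cast, passing negated attack damage as a set-by-caller Health magnitude, then ends.
; Left and right fire montage nodes exist but are unconnected.
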(event Ability|EventActivateAbility
  (Development|PrintString "Primary Attack")
  (bind _asbp_chtwinblast (Utilities|Casting|CastToBP_CHTwinblast (Variables|Default|GetCharacterRef)))
  (Variables|Default|SetTwinblastChar _asbp_chtwinblast)
  (Ability|CommitAbility))

(event Ability|EventCommitExecute
  (bind _twinblastchar (Variables|Default|GetTwinblastChar))
  (bind _abilitysystemcomponent (Variables|/Script/MobaProject.CHBase|GetAbilitySystemComponent _twinblastchar))
  (Class|CHGameplayAbility|RotateCharacter (.Yaw (Math|Rotator|BreakRotator (Math|Rotator|FindLookatRotation (Transformation|GetActorLocation (Variables|Default|GetTwinblastChar)) (Transformation|GetActorLocation (Variables|/Script/MobaProject.CHPlayable|GetPrimaryAttackTarget (Variables|Default|GetTwinblastChar)))))))
  (bind _returnvalue (Class|CHPlayable|GetPrimaryAttackDamage _twinblastchar))
  (bind _returnvalue_2 (Ability|GameplayEffect|AssignTagSetbyCallerMagnitude (GameplayEffects|MakeOutgoingSpec _abilitysystemcomponent "/Game/Blueprints/Characters/Playable/Twinblast/Abilities/PrimaryAttack/GE_TwinblastPrimaryAttackDamage.GE_TwinblastPrimaryAttackDamage_C" 0.0 (GameplayEffects|MakeEffectContext _abilitysystemcomponent)) "(TagName=\"setByCallerTag.Health\")" (* _returnvalue -1.0)))
  (bind _ascan_take_damage (Utilities|Casting|CastToCanTakeDamage (Variables|/Script/MobaProject.CHPlayable|GetPrimaryAttackTarget (Variables|Default|GetTwinblastChar))))
  (bind _returnvalue_3 (Class|CanTakeDamage|GetAbilitySystem _ascan_take_damage))
  (GameplayEffects|ApplyGameplayEffectSpecToTarget _abilitysystemcomponent _returnvalue_2 _returnvalue_3)
  (Ability|EndAbility))